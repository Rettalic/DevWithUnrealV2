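; BP_NPC is a talkable NPC that shows dialogue lines in a UI_Dialogue widget.
; Each Talk call advances an index through the Dialogue array, then loops or jumps to SummaryIndex after the last line.
; Trigger overlap begin jumps into Talk's widget-creation and text path without advancing, while overlap end removes the widget and resets the index.
; Disconnected debug print and duplicate Talk logic remain in the graph.
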(event OnComponentEndOverlap(Trigger)
  (params (OverlappedComponent :type Primitive%20Component%20Object%20Reference) (OtherActor :type Actor%20Object%20Reference) (OtherComp :type Primitive%20Component%20Object%20Reference) (OtherBodyIndex :type Integer))
  (Widget|RemovefromParent (Variables|Default|GetUI))
  (Variables|Default|SetTalkIndex -1))

(event OnComponentBeginOverlap(Trigger)
  (params (OverlappedComponent :type Primitive%20Component%20Object%20Reference) (OtherActor :type Actor%20Object%20Reference) (OtherComp :type Primitive%20Component%20Object%20Reference) (OtherBodyIndex :type Integer) (bFromSweep :type Boolean) (SweepResult :type Hit%20Result%20Structure%20%28by%20ref%29))
  (bind _dialogue (Variables|Default|GetDialogue))
  (bind _returnvalue (Utilities|Array|LastIndex _dialogue))
  (bind _returnvalue_2 (UserInterface|CreateWidget "/Game/DialogueSystem/UI_Dialogue.UI_Dialogue_C"))
  (bind _output_get (Variables|Default|SetUI _returnvalue_2))
  (UserInterface|Viewport|AddtoViewport _output_get 0)
  (Rendering|Components|TextRender|SetText (Variables|/Game/DialogueSystem/UI_Dialogue.UI_Dialogue_C|GetTalkText (Variables|Default|GetUI)) (Utilities|Text|ToText(String) (Utilities|Array|Get(acopy) (Variables|Default|GetDialogue) (Variables|Default|GetTalkIndex))))
  (bind _output_get_2 (Variables|Default|SetIsDone (== (Variables|Default|GetTalkIndex) _returnvalue)))
  (if _output_get_2
    (Variables|Default|SetTalkIndex _returnvalue)
    (if (Variables|Default|GetDialogueIsloopable)
      (Variables|Default|SetTalkIndex -1)
      (else
        (Variables|Default|SetTalkIndex (Variables|Default|GetSummaryIndex))))))

(event EventTalk
  (bind _dialogue (Variables|Default|GetDialogue))
  (bind _returnvalue (Utilities|Array|LastIndex _dialogue))
  (Math|Integer|IncrementInt (Variables|Default|GetTalkIndex)
    (:%20%20
      (if (< (Variables|Default|GetTalkIndex) (Utilities|Array|Length (Variables|Default|GetDialogue)))
        (Variables|Default|GetUI
          (:then
            _)
          (:else
            (bind _returnvalue_2 (UserInterface|CreateWidget "/Game/DialogueSystem/UI_Dialogue.UI_Dialogue_C"))
            (bind _output_get (Variables|Default|SetUI _returnvalue_2))
            (UserInterface|Viewport|AddtoViewport _output_get 0)))
        (Rendering|Components|TextRender|SetText (Variables|/Game/DialogueSystem/UI_Dialogue.UI_Dialogue_C|GetTalkText (Variables|Default|GetUI)) (Utilities|Text|ToText(String) (Utilities|Array|Get(acopy) (Variables|Default|GetDialogue) (Variables|Default|GetTalkIndex))))
        (bind _output_get_2 (Variables|Default|SetIsDone (== (Variables|Default|GetTalkIndex) _returnvalue)))
        (if _output_get_2
          (Variables|Default|SetTalkIndex _returnvalue)
          (if (Variables|Default|GetDialogueIsloopable)
            (Variables|Default|SetTalkIndex -1)
            (else
              (Variables|Default|SetTalkIndex (Variables|Default|GetSummaryIndex)))))
        (else
          (Widget|RemovefromParent (Variables|Default|GetUI)))))))

(fn ConstructionScript)